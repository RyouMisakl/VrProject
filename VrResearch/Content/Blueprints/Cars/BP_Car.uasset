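; BP_Car is a car moved by a PFPathFollower component that slows or halts when another BP_Car is near.
; Its SlowZone and StopZone components detect other cars through overlap events and set the follower's SpeedDuration to a reduced value or zero.
; Ending either overlap restores the same default value, without checking whether the other zone or another car still overlaps.
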(event OnComponentBeginOverlap(SlowZone)
  (params (OverlappedComponent :type Primitive%20Component%20Object%20Reference) (OtherActor :type Actor%20Object%20Reference) (OtherComp :type Primitive%20Component%20Object%20Reference) (OtherBodyIndex :type Integer) (bFromSweep :type Boolean) (SweepResult :type Hit%20Result%20Structure%20%28by%20ref%29))
  (Utilities|Casting|CastToBP_Car OtherActor)
  (Variables|/Script/PathFollow.PFPathFollowerComponent|SetSpeedDuration (Variables|Default|GetPFPathFollower) 2e+01))

(event OnComponentEndOverlap(SlowZone)
  (params (OverlappedComponent :type Primitive%20Component%20Object%20Reference) (OtherActor :type Actor%20Object%20Reference) (OtherComp :type Primitive%20Component%20Object%20Reference) (OtherBodyIndex :type Integer))
  (Utilities|Casting|CastToBP_Car OtherActor)
  (Variables|/Script/PathFollow.PFPathFollowerComponent|SetSpeedDuration (Variables|Default|GetPFPathFollower) 8e+02))

(event OnComponentBeginOverlap(StopZone)
  (params (OverlappedComponent :type Primitive%20Component%20Object%20Reference) (OtherActor :type Actor%20Object%20Reference) (OtherComp :type Primitive%20Component%20Object%20Reference) (OtherBodyIndex :type Integer) (bFromSweep :type Boolean) (SweepResult :type Hit%20Result%20Structure%20%28by%20ref%29))
  (Utilities|Casting|CastToBP_Car OtherActor)
  (Variables|/Script/PathFollow.PFPathFollowerComponent|SetSpeedDuration (Variables|Default|GetPFPathFollower) 0.0))

(event OnComponentEndOverlap(StopZone)
  (params (OverlappedComponent :type Primitive%20Component%20Object%20Reference) (OtherActor :type Actor%20Object%20Reference) (OtherComp :type Primitive%20Component%20Object%20Reference) (OtherBodyIndex :type Integer))
  (Utilities|Casting|CastToBP_Car OtherActor)
  (Variables|/Script/PathFollow.PFPathFollowerComponent|SetSpeedDuration (Variables|Default|GetPFPathFollower) 8e+02))

(event EventBeginPlay)

(event Collision|EventActorBeginOverlap
  (params (OtherActor :type Actor%20Object%20Reference)))

(event EventTick
  (params (DeltaSeconds :type Float%20%28single-precision%29)))

(fn ConstructionScript)